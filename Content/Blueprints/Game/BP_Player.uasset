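; BP_Player turns number key presses (0–9) into movement commands for the BP_Item actors in the level.
; On BeginPlay it caches every BP_Item in an array.
; Each key press converts the key's display name to an integer and tells the item with that index to move to its selected position.
; The MoveAllItemsAtOnce flag decides whether only the first match or every matching item moves.
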(event `self.ReceiveBeginPlay`
  ;[0.2753 0.2077 1] Initialization
  (`self.Set Items Array`))

(event `Key|Zero`
  (params (Key :type "Key Structure"))
  ;[1 1 1] Player Input
  (:`Pressed`
    (`self.Move Relevant Item` Key)))

(event `Key|Five`
  (params (Key :type "Key Structure"))
  ;[1 1 1] Player Input
  (:`Pressed`
    (`self.Move Relevant Item` Key)))

(event `Key|One`
  (params (Key :type "Key Structure"))
  ;[1 1 1] Player Input
  (:`Pressed`
    (`self.Move Relevant Item` Key)))

(event `Key|Six`
  (params (Key :type "Key Structure"))
  ;[1 1 1] Player Input
  (:`Pressed`
    (`self.Move Relevant Item` Key)))

(event `Key|Two`
  (params (Key :type "Key Structure"))
  ;[1 1 1] Player Input
  (:`Pressed`
    (`self.Move Relevant Item` Key)))

(event `Key|Seven`
  (params (Key :type "Key Structure"))
  ;[1 1 1] Player Input
  (:`Pressed`
    (`self.Move Relevant Item` Key)))

(event `Key|Three`
  (params (Key :type "Key Structure"))
  ;[1 1 1] Player Input
  (:`Pressed`
    (`self.Move Relevant Item` Key)))

(event `Key|Eight`
  (params (Key :type "Key Structure"))
  ;[1 1 1] Player Input
  (:`Pressed`
    (`self.Move Relevant Item` Key)))

(event `Key|Nine`
  (params (Key :type "Key Structure"))
  ;[1 1 1] Player Input
  (:`Pressed`
    (`self.Move Relevant Item` Key)))

(event `Key|Four`
  (params (Key :type "Key Structure"))
  ;[1 1 1] Player Input
  (:`Pressed`
    (`self.Move Relevant Item` Key)))

(fn `Move Relevant Item`
  (params (Key :type "Key Structure (by ref)"))
  (for _array_element (`self.BP_Items`)
    (`/Engine/EditorBlueprintResources/StandardMacros.IsValid` _array_element
      (:`Is Valid`
        (if (== (`/Game/Blueprints/Actors/BP_Item.Get Index` _array_element) (`KismetStringLibrary.Conv_StringToInt` (`KismetTextLibrary.Conv_TextToString` (`KismetInputLibrary.Key_GetDisplayName` Key false))))
          (`/Game/Blueprints/Actors/BP_Item.Move To Selected Pos` _array_element)
          (if (not (`self.bMoveAllItemsAtOnce`))
            (break)))))))

(fn `Set Items Array`
  (bind _outactors (`GameplayStatics.GetAllActorsOfClass` "/Game/Blueprints/Actors/BP_Item.BP_Item_C"))
  (set `self.BP_Items` _outactors))

(fn `UserConstructionScript`)