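; BP_Item is a numbered item that moves to one of two randomly chosen BP_Boxes positions and drops into a box.
; MoveToSelectedPos drives an InterpTo movement component; on stop, it enables physics if Distance is near zero, otherwise moves again.
; Three seconds later, an item not destroyed by box overlap replaces itself at its start point with the same Index.
; It then has BP_Player rebuild its items array.
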(event `self.ReceiveBeginPlay`
  ;[0.2753 0.2077 1] Initialization
  (`self.Find and Set BP Boxes Ref`)
  (`self.Set Random Pos`)
  (set `self.Starting Point` (`self.K2_GetActorLocation`)))

(event `self.Movement Component.OnInterpToStop`
  (params (ImpactResult :type "HitResult Structure (by ref)") (Time :type "Float (single-precision)"))
  ;[1 1 1] On Movement Stop
  (`self.Drop Item Into A Box` ImpactResult_Distance)
  ;[1 1 1] Wait And..
  (`KismetSystemLibrary.Delay` 3.0)
  ;[1 1 1] Respawn If Not Destroyed (Didn't Ovelapped Box Collision)
  (`self.Respawn Item`)
  (`self.Reset Items Array On BP Player`))

(fn `Drop Item Into A Box`
  (params (`Distance To Box` :type "Float (double-precision)"))
  (if (< `Distance To Box` 0.5)
    (`PrimitiveComponent.SetCollisionEnabled` (`self.Mesh`) "QueryAndPhysics")
    (`PrimitiveComponent.SetSimulatePhysics` (`self.Mesh`) true)
    (else
      (`self.Move To Selected Pos`))))

(fn `Find and Set BP Boxes Ref`
  (bind _returnvalue (`GameplayStatics.GetActorOfClass` "/Game/Blueprints/Actors/BP_Boxes.BP_Boxes_C"))
  (set `self.Bp_Boxes` _returnvalue))

(fn `Get Index`
  (returns (Index :type Integer))
  (return (`self.Index`)))

(fn `Move To Selected Pos`
  (bind _bp_boxes (`self.Bp_Boxes`)
    (:`then`
      (`InterpToMovementComponent.AddControlPointPosition` (`self.Movement Component`) (`/Game/Blueprints/Actors/BP_Boxes.Get Pos Location` _bp_boxes (`self.bIsFirstPos`)) false)
      (`ActorComponent.SetActive` (`self.Movement Component`) true true))
    (:`else`)))

(fn `Reset Items Array On BP Player`
  (bind _asbp_player (cast `/Game/Blueprints/Game/BP_Player` (`GameplayStatics.GetPlayerPawn` 0)))
  (`/Game/Blueprints/Game/BP_Player.Set Items Array` _asbp_player))

(fn `Respawn Item`
  (`self.K2_DestroyActor`)
  (`|SpawnActorFromClass` "BP_Item_C" (`KismetMathLibrary.MakeTransform` (`self.Starting Point`)) "Undefined" "OverrideRootScale" null (`self.Index`) null))

(fn `Set Index Text`
  (`TextRenderComponent.K2_SetText` (`self.IndexText`) (`KismetTextLibrary.Conv_IntToText` (`self.Index`))))

(fn `Set Random Pos`
  (set `self.bIsFirstPos` (`KismetMathLibrary.RandomBool`)))

(fn `UserConstructionScript`
  (`self.Set Index Text`))