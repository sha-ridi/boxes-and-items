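; BP_Boxes is an actor with two collision boxes that destroy tagged actors entering them.
; Begin-overlap events on both boxes feed a shared function that destroys the other actor if it is valid and tagged "Destructible".
; GetPosLocation returns the world location of either Pos1 or Pos2, chosen by a boolean, though nothing in this Blueprint calls it.
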(event `self.BoxCollision.OnComponentBeginOverlap`
  (params (OverlappedComponent :type "PrimitiveComponent Object Reference") (OtherActor :type "Actor Object Reference") (OtherComp :type "PrimitiveComponent Object Reference") (OtherBodyIndex :type Integer) (bFromSweep :type Boolean) (SweepResult :type "HitResult Structure (by ref)"))
  ;[1 1 1] On Box Collisions Overlapped
  (`self.Destroy Other Actor If Possible` OtherActor))

(event `self.BoxCollision2.OnComponentBeginOverlap`
  (params (OverlappedComponent :type "PrimitiveComponent Object Reference") (OtherActor :type "Actor Object Reference") (OtherComp :type "PrimitiveComponent Object Reference") (OtherBodyIndex :type Integer) (bFromSweep :type Boolean) (SweepResult :type "HitResult Structure (by ref)"))
  ;[1 1 1] On Box Collisions Overlapped
  (`self.Destroy Other Actor If Possible` OtherActor))

(fn `Destroy Other Actor If Possible`
  (params (Actor :type "Actor Object Reference"))
  (`/Engine/EditorBlueprintResources/StandardMacros.IsValid` Actor
    (:`Is Valid`
      (if (`self.ActorHasTag` Actor "Destructible")
        (`self.K2_DestroyActor` Actor)))))

(fn `Get Pos Location`
  (params (bIsFirstPos :type Boolean))
  (returns (`Pos Location` :type "Vector Structure"))
  (return (`SceneComponent.K2_GetComponentLocation` (select `bool` bIsFirstPos :`false` (`self.Pos2`) :`true` (`self.Pos1`)))))

(fn `UserConstructionScript`)